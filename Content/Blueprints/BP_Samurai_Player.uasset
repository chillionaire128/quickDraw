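; BP_Samurai_Player is the player-controlled samurai, set up with duel input and a level camera view.
; On BeginPlay it has the first player controller possess it, adds the IMC_Duel Enhanced Input mapping context, and switches the view to a CameraActor found in the level.
; The IA_Attack input only prints a debug string, with no attack logic in this graph yet.
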(event `self.ReceiveBeginPlay`
  (`parent.ReceiveBeginPlay`)
  (`Controller.Possess` (`GameplayStatics.GetPlayerController` 0) self)
  (bind _asplayer_controller (cast `PlayerController` (`self.GetController`)))
  (`EnhancedInputSubsystemInterface.AddMappingContext` (pcsubsystem `EnhancedInputLocalPlayerSubsystem` _asplayer_controller) "/Game/input/IMC_Duel.IMC_Duel" 0 (struct))
  (bind _returnvalue (`GameplayStatics.GetActorOfClass` "/Script/Engine.CameraActor"))
  (`PlayerController.SetViewTargetWithBlend` (`GameplayStatics.GetPlayerController` 0) _returnvalue 0.0 "VTBlend_Linear" 0.0 false))

(event `EnhancedInput|/Game/input/Actions/IA_Attack`
  (params (ActionValue :type Boolean) (ElapsedSeconds :type "Float (double-precision)") (TriggeredSeconds :type "Float (double-precision)") (InputAction :type "InputAction Object Reference" :default "/Game/input/Actions/IA_Attack.IA_Attack"))
  (:`Started`
    (`KismetSystemLibrary.PrintString` "Attack")))

(fn `UserConstructionScript`
  (`parent.UserConstructionScript`))