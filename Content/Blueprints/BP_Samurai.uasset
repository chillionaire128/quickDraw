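; BP_Samurai is a samurai Blueprint with a timeline-driven slide-in animation for its primary sprite.
; BeginPlay caches the sprite's relative location as its resting position, then calls SlideIn, whose body is not in this graph.
; A separate SlideExample event plays the SlideInAnim timeline at double rate, lerping the sprite from SlideStartPos to that cached position.
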(event `self.ReceiveBeginPlay`
  (set `self.SpriteDefaultPos` (`SceneComponent.RelativeLocation` (`self.PrimarySprite`)))
  (`self.SlideIn`))

(event `SlideExample`
  (`TimelineComponent.SetPlayRate` (`self.SlideInAnim`) 2.0)
  (bind (_direction _alpha) (`Timeline|SlideInAnim`)
    (:`Update`
      (`SceneComponent.K2_SetRelativeLocation` (`self.PrimarySprite`) (`KismetMathLibrary.VLerp` (`self.SlideStartPos`) (`self.SpriteDefaultPos`) _alpha) false false))))

(fn `UserConstructionScript`)